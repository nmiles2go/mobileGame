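; Puzzle player character Blueprint that handles jump input and carries a selection cursor widget component to show or hide a selection indicator.
; EnableSelectionWidget shows the cursor and loops its WBP_SelectionIcon animation indefinitely, while DisableSelectionWidget stops the animation and hides it.
; The cursor is disabled on BeginPlay, and nothing in this Blueprint calls the enable function.
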(event `self.ReceiveBeginPlay`
  (`self.DisableSelectionWidget`))

(event `InputAction|Jump`
  (params (Key :type "Key Structure"))
  (:`Pressed`
    (`self.Jump`)))

(fn `DisableSelectionWidget`
  (bind _selectioncursor (`self.SelectionCursor`))
  (bind _aswbp_selection_icon (cast `/Game/Blueprints/HUD/WBP_SelectionIcon` (`WidgetComponent.GetUserWidgetObject` _selectioncursor)))
  (`UserWidget.StopAnimation` _aswbp_selection_icon (`/Game/Blueprints/HUD/WBP_SelectionIcon.CursorAnimation` _aswbp_selection_icon))
  (`SceneComponent.SetVisibility` _selectioncursor false false))

(fn `EnableSelectionWidget`
  (bind _selectioncursor (`self.SelectionCursor`))
  (bind _aswbp_selection_icon (cast `/Game/Blueprints/HUD/WBP_SelectionIcon` (`WidgetComponent.GetUserWidgetObject` _selectioncursor)))
  (`UserWidget.PlayAnimation` _aswbp_selection_icon (`/Game/Blueprints/HUD/WBP_SelectionIcon.CursorAnimation` _aswbp_selection_icon) 0.0 0 "Forward" 1.0 false)
  (`SceneComponent.SetVisibility` _selectioncursor true false))

(fn `UserConstructionScript`)