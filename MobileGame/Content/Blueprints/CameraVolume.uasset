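; Camera volume actor that takes over the player's view when the puzzle player character enters its box.
; On overlap it stores the character, registers itself as the character's current camera volume and blends the player controller's view target to itself with a cubic ease.
; When spline mode is enabled, each tick turns the camera toward the character and slides it to the closest spline point to them, giving a rail-style follow camera.
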(event `self.ReceiveBeginPlay`
  (set `self.Controller` (`GameplayStatics.GetPlayerController` 0)))

(event `self.Box.OnComponentBeginOverlap`
  (params (OverlappedComponent :type "PrimitiveComponent Object Reference") (OtherActor :type "Actor Object Reference") (OtherComp :type "PrimitiveComponent Object Reference") (OtherBodyIndex :type Integer) (bFromSweep :type Boolean) (SweepResult :type "HitResult Structure (by ref)"))
  (bind _controller (`self.Controller`))
  (bind _aspc_puzzle_player_character (cast `/Game/Blueprints/Character/PC_PuzzlePlayerCharacter` OtherActor))
  (bind _output_get (set `self.character` _aspc_puzzle_player_character))
  (set `/Game/Blueprints/Character/PC_PuzzlePlayerCharacter.CurrentCameraVolume` self _output_get)
  (`/Engine/EditorBlueprintResources/StandardMacros.IsValid` _controller
    (:`Is Valid`
      (`PlayerController.SetViewTargetWithBlend` _controller self 2.0 "VTBlend_Cubic" 0.0 false))))

(event `self.ReceiveTick`
  (params (DeltaSeconds :type "Float (single-precision)"))
  (bind _camera (`self.Camera`))
  (bind _returnvalue (`self.K2_GetActorLocation` (`self.character`)))
  (if (`self.UseSpline`)
    (`/Engine/EditorBlueprintResources/StandardMacros.IsValid` (`self.character`)
      (:`Is Valid`
        (`SceneComponent.K2_SetWorldRotation` _camera (`KismetMathLibrary.FindLookAtRotation` (`SceneComponent.K2_GetComponentLocation` (`self.Camera`)) _returnvalue) false false)
        (`SceneComponent.K2_SetWorldLocation` _camera (`SplineComponent.FindLocationClosestToWorldLocation` (`self.Spline`) _returnvalue "World") false false)))))

(fn `UserConstructionScript`)